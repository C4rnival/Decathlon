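; Clickable sports card actor that takes its name and color from DT_SportCards and switches between Hand and Board states.
; Hovering in Hand lifts and enlarges it, and unhovering also disables mouse-over events after a short delay.
; Clicking toggles selection by state, with deselection returning it to its BeginPlay location.
; Gated Tick cursor-follow exists, but its press, release and board-snap logic is disconnected, and oscillation is an empty stub.
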(event `self.ReceiveBeginPlay`
  (`self.SetCardStartingPosition`))

(event `CardOscillation`
  ;[1 1 1] Oscillazione carta (stile Balatro) ((aggiungere posizione di partenza carta))
)

(event `self.CardBase.OnBeginCursorOver`
  (params (TouchedComponent :type "PrimitiveComponent Object Reference"))
  (switch `/Game/Cards/ECard_State` (`self.cardStateSelection`)
    (:`NewEnumerator1`
      (`self.OnCardStartHover`))))

(event `self.CardBase.OnEndCursorOver`
  (params (TouchedComponent :type "PrimitiveComponent Object Reference"))
  (switch `/Game/Cards/ECard_State` (`self.cardStateSelection`)
    (:`NewEnumerator1`
      (`self.OnCardStopHover`)
      (`KismetSystemLibrary.K2_SetTimer` self "DisableMouseEvents" 0.25))))

(event `self.CardBase.OnClicked`
  (params (TouchedComponent :type "PrimitiveComponent Object Reference") (ButtonPressed :type "Key Structure"))
  (switch `/Game/Cards/ECard_State` (`self.cardStateSelection`)
    (:`NewEnumerator1`
      (`self.SelectCard`))
    (:`NewEnumerator3`
      (`self.DeselectCard`))))

(event `self.CardBase.OnReleased`
  (params (TouchedComponent :type "PrimitiveComponent Object Reference") (ButtonReleased :type "Key Structure")))

(event `self.ReceiveTick`
  (params (DeltaSeconds :type "Float (single-precision)"))
  (bind (_cardpreviouslocation_x _cardpreviouslocation_y _cardpreviouslocation_z) (`KismetMathLibrary.BreakVector` (`self.cardPreviousLocation`)))
  (`/Engine/EditorBlueprintResources/StandardMacros.Gate` true :!label _label
    (:`Exit`
      (`self.K2_SetActorLocation` (`KismetMathLibrary.VInterpTo` (`self.K2_GetActorLocation`) (`KismetMathLibrary.MakeVector` (.x (`.Location` (`GameplayStatics.BreakHitResult` (`PlayerController.GetHitResultUnderCursorByChannel` (`GameplayStatics.GetPlayerController` 0) "TraceTypeQuery1" true)))) (.y (`.Location` (`GameplayStatics.BreakHitResult` (`PlayerController.GetHitResultUnderCursorByChannel` (`GameplayStatics.GetPlayerController` 0) "TraceTypeQuery1" true)))) _cardpreviouslocation_z) (`GameplayStatics.GetWorldDeltaSeconds`) 12.0))
      (`self.K2_SetActorRotation` (`self.K2_GetActorRotation`)))))

(event `OpenClickGate`
  (`/Engine/EditorBlueprintResources/StandardMacros.Gate` false :!via `Open` :!label _label_2
    (:`Exit`
      (set `self.isMouseReleased` false)
      (goto _label :!via `Open`))))

(event `CloseOnClickGate`
  (goto _label_2 :!via `Close`))

(event `CloseGate`
  (goto _label :!via `Close`))

(fn `ActivateMouseEvents`
  (set `PlayerController.bEnableMouseOverEvents` true (`GameplayStatics.GetPlayerController` 0)))

(fn `CanPlaceCardOnBoard`
  (params (State :type "/Game/Cards/ECard_State Enum" :default "NewEnumerator0"))
  (returns (ReturnValue :type Boolean))
  (set `self.cardStateSelection` State)
  (return false))

(fn `DeselectCard`
  (if (`self.cardHovered`)
    (if (`self.cardSelected`)
      (`self.K2_TeleportTo` (`self.cardPreviousLocation`) (`self.K2_GetActorRotation`))
      (`SceneComponent.SetWorldScale3D` (`self.DefaultSceneRoot`) (0.4 0.4 0.4))
      (set `self.cardSelected` false)
      (set `self.cardStateSelection` "NewEnumerator1"))))

(fn `DisableMouseEvents`
  (set `PlayerController.bEnableMouseOverEvents` false (`GameplayStatics.GetPlayerController` 0)))

(fn `OnCardClick`
  (if (== (`GameplayStatics.GetObjectClass` (`.HitActor` (`GameplayStatics.BreakHitResult` (`PlayerController.GetHitResultUnderCursorByChannel` (`GameplayStatics.GetPlayerController` 0) "TraceTypeQuery1" true)))) "/Game/Personal/BP_CartaMaster.BP_CartaMaster_C")
    _
    (else
      _))
  (`KismetSystemLibrary.PrintString` "Hello"))

(fn `OnCardReleaseClick`
  (if (== (`GameplayStatics.GetObjectClass` (`.HitActor` (`GameplayStatics.BreakHitResult` (`PlayerController.GetHitResultUnderCursorByChannel` (`GameplayStatics.GetPlayerController` 0) "TraceTypeQuery1" true)))) "/Game/Personal/BP_CartaMaster.BP_CartaMaster_C")
    _))

(fn `OnCardStartHover`
  (if (not (`self.cardHovered`))
    (`self.K2_TeleportTo` (+ (`SceneComponent.K2_GetComponentLocation` (`self.CardBase`)) (`self.HoverOffset`)) (`self.K2_GetActorRotation`))
    (`SceneComponent.SetWorldScale3D` (`self.DefaultSceneRoot`) (0.6 0.6 0.6))
    (set `self.cardHovered` true)))

(fn `OnCardStopHover`
  (if (`self.cardHovered`)
    (if (not (`self.cardSelected`))
      (`self.K2_TeleportTo` (- (`SceneComponent.K2_GetComponentLocation` (`self.CardBase`)) (`self.HoverOffset`)) (`self.K2_GetActorRotation`))
      (switch `/Game/Cards/ECard_State` (`self.cardStateSelection`)
        (:`NewEnumerator1`
          (`SceneComponent.SetWorldScale3D` (`self.DefaultSceneRoot`) (0.4 0.4 0.4))
          (set `self.cardHovered` false))))))

(fn `PlaceCardOnBoard`
  (params (PlaceLocation :type "Vector Structure"))
  (returns (ReturnValue :type Boolean))
  (set `self.boardPlaceLocation` PlaceLocation)
  (return false))

(fn `SelectCard`
  (if (`self.cardHovered`)
    (`self.K2_TeleportTo` (`SceneComponent.K2_GetComponentLocation` (`self.CardBase`)) (`self.K2_GetActorRotation`))
    (set `self.cardSelected` true)
    (set `self.cardStateSelection` "NewEnumerator3")))

(fn `SetCardData`
  (params (RowName :type Name))
  (bind _returnvalue (`|GetDataTableRow` "/Game/Manage/CardsData/DT_SportCards.DT_SportCards" RowName)
    (:`then`
      (set `self.cardSportName` (`KismetTextLibrary.Conv_NameToText` RowName))
      (set `self.cardSportColor` (`.Color_7_F1884BF94702D8EA9AC7B79B54B96B53` (break `/Game/Manage/CardsData/STR_SportCard` _returnvalue)))
      (`self.UpdateCardData`))))

(fn `SetCardStartingPosition`
  (set `self.cardPreviousLocation` (`SceneComponent.K2_GetComponentLocation` (`self.CardBase`))))

(fn `SetCardState`)

(fn `UpdateCardData`
  (bind (_cardsportcolor_b _cardsportcolor_g _cardsportcolor_r) (break `Color` (`self.cardSportColor`)))
  (`TextRenderComponent.K2_SetText` (`self.TextRender`) (`self.cardSportName`))
  (`MeshComponent.SetVectorParameterValueOnMaterials` (`self.CardBase`) "cardColor" (`KismetMathLibrary.ClampVectorSize` (`KismetMathLibrary.MakeVector` (`KismetMathLibrary.Conv_ByteToDouble` _cardsportcolor_r) (`KismetMathLibrary.Conv_ByteToDouble` _cardsportcolor_g) (`KismetMathLibrary.Conv_ByteToDouble` _cardsportcolor_b)) 1.0 1.0)))

(fn `UserConstructionScript`)