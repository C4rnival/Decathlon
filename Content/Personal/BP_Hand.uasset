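; BP_Hand is an actor that lays out a hand of sport cards in the world as a row of spawned actors.
; It records its location on BeginPlay, then SpawnCardInit stores the given card array and calls SpawnCard for each entry.
; SpawnCard spawns the card's class with its sport-card struct at a fixed rotation, spaced by index, with the start X and Y swapped.
; AddCardInit repeats the same layout logic inline.
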(event `self.ReceiveBeginPlay`
  (set `self.Start` (`self.K2_GetActorLocation`)))

(event `SpawnCardInit`
  (params (Mano :type "Array of /Game/Personal/BP_Card Object Reference"))
  (bind _output_get (set `self.Mano` Mano))
  (for (_array_element _array_index) _output_get
    (`self.SpawnCard` _array_element _array_index)))

(fn `Add CardInit`
  (params (Mano :type "Array of /Game/Personal/BP_Card Object Reference"))
  (bind (_start_x _start_y _start_z) (`KismetMathLibrary.BreakVector` (`self.Start`)))
  (bind _output_get (set `self.Mano` Mano))
  (for (_ _array_index) _output_get
    (bind _output (`|GetArrayItem` _output_get _array_index))
    (`|SpawnActorFromClass` (`GameplayStatics.GetObjectClass` _output) (`KismetMathLibrary.MakeTransform` (`KismetMathLibrary.MakeVector` _start_y (+ _start_x (* _array_index 75.0)) _start_z) (struct :`Pitch` 90.0 :`Yaw` 180.0)) "Undefined" "OverrideRootScale" null (`/Game/Personal/BP_CartaMaster.STR_SportCard` _output) null)))

(fn `SpawnCard`
  (params (Card :type "/Game/Personal/BP_Card Object Reference") (Index :type Integer))
  (bind (_start_x _start_y _start_z) (`KismetMathLibrary.BreakVector` (`self.Start`)))
  (`|SpawnActorFromClass` (`GameplayStatics.GetObjectClass` Card) (`KismetMathLibrary.MakeTransform` (`KismetMathLibrary.MakeVector` _start_y (+ _start_x (* Index 75.0)) _start_z) (struct :`Pitch` 90.0 :`Yaw` 180.0)) "Undefined" "OverrideRootScale" null (`/Game/Personal/BP_CartaMaster.STR_SportCard` Card) null))

(fn `UserConstructionScript`)