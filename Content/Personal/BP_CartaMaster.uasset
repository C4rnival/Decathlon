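; Base card actor for a sports card game, with a text label showing its sport and a data table lookup for name and color.
; Hovering a hand card lifts and enlarges it, with paired DoOnce gates preventing repeat triggers.
; FInteract toggles zoom and registers the card in the player controller's selection, capped at three.
; Click and board-placement functions are mostly stubs that print or store state.
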(event `self.Card0.OnBeginCursorOver`
  (params (TouchedComponent :type "PrimitiveComponent Object Reference"))
  (`/Engine/EditorBlueprintResources/StandardMacros.DoOnce` false :!label _label
    (:`Completed`
      (switch `/Game/Cards/ECard_State` (`self.cardStateSelection`)
        (:`NewEnumerator1`
          (`self.OnCardStartHover`)
          (`self.ResetDoOnceNotOver`))))))

(event `ResetDoOnceHover`
  (goto _label :!via `Reset`))

(event `self.Card0.OnEndCursorOver`
  (params (TouchedComponent :type "PrimitiveComponent Object Reference"))
  (switch `/Game/Cards/ECard_State` (`self.cardStateSelection`)
    (:`NewEnumerator1`
      (`/Engine/EditorBlueprintResources/StandardMacros.DoOnce` false :!label _label_2
        (:`Completed`
          (`self.ResetDoOnceHover`)
          (`self.OnCardStopHover`)
          (`self.ActivateMouseEvents`))))))

(event `ResetDoOnceNotOver`
  (goto _label_2 :!via `Reset`))

(event `ZoomIn`
  (`self.SetActorScale3D` (2.0 2.0 2.0))
  (set `self.IsZoomIn?` true))

(event `self.ReceiveBeginPlay`
  (`self.UpdateCardData`)
  (bind _asbp_player_controller (cast `/Game/Personal/BP_PlayerController` (`GameplayStatics.GetPlayerController` 0)))
  (set `self.As BP Player Controller` _asbp_player_controller))

(event `ZoomOut`
  (`self.SetActorScale3D` (1.0 1.0 1.0))
  (set `self.IsZoomIn?` false))

(event `/Game/Personal/BPI_Interaction.F_Interact`
  (params (SelectedCard :type Integer))
  (bind _as_bp_player_controller (`self.As BP Player Controller`))
  (bind _selectedcardarray (`/Game/Personal/BP_PlayerController.SelectedCardArray` _as_bp_player_controller))
  (bind _selectedcard (`/Game/Personal/BP_PlayerController.SelectedCard` _as_bp_player_controller))
  (if (`self.IsZoomIn?`)
    (`self.ZoomOut`)
    (`/Engine/EditorBlueprintResources/StandardMacros.DecrementInt` _selectedcard
      (:`  `
        (`KismetArrayLibrary.Array_RemoveItem` _selectedcardarray self)))
    (elif (< SelectedCard 3)
      (`self.ZoomIn`)
      (`/Engine/EditorBlueprintResources/StandardMacros.IncrementInt` _selectedcard
        (:`  `
          (`KismetArrayLibrary.Array_Add` _selectedcardarray self)
          (`/Game/Personal/BP_PlayerController.ControlNCard` _as_bp_player_controller))))))

(fn `ActivateMouseEvents`
  (bind _returnvalue (`GameplayStatics.GetPlayerController` 0))
  (`/Engine/EditorBlueprintResources/StandardMacros.FlipFlop`
    (:`A`
      (set `PlayerController.bEnableMouseOverEvents` true _returnvalue))
    (:`B`
      (set `PlayerController.bEnableMouseOverEvents` false _returnvalue))))

(fn `CanPlaceCardOnBoard`
  (params (State :type "/Game/Cards/ECard_State Enum" :default "NewEnumerator0"))
  (returns (ReturnValue :type Boolean))
  (set `self.cardStateSelection` State)
  (return false))

(fn `OnCardClick`
  (if (== (`GameplayStatics.GetObjectClass` (`.HitActor` (`GameplayStatics.BreakHitResult` (`PlayerController.GetHitResultUnderCursorByChannel` (`GameplayStatics.GetPlayerController` 0) "TraceTypeQuery1" true)))) "BP_CartaMaster_C")
    _
    (else
      _))
  (`KismetSystemLibrary.PrintString` "Hello"))

(fn `OnCardReleaseClick`
  (if (== (`GameplayStatics.GetObjectClass` (`.HitActor` (`GameplayStatics.BreakHitResult` (`PlayerController.GetHitResultUnderCursorByChannel` (`GameplayStatics.GetPlayerController` 0) "TraceTypeQuery1" true)))) "BP_CartaMaster_C")
    _))

(fn `OnCardStartHover`
  (bind _card0 (`self.Card0`))
  (`SceneComponent.K2_SetWorldLocation` _card0 (+ (`|GetArrayItem` (`self.Array_Billboard`)) (`self.HoverOffset`)) true true)
  (`SceneComponent.SetWorldScale3D` _card0 (1.6 1.6 1.6))
  (`KismetSystemLibrary.PrintString` "FineDentro"))

(fn `OnCardStopHover`
  (bind _card0 (`self.Card0`))
  (`SceneComponent.K2_SetWorldLocation` _card0 (- (`|GetArrayItem` (`self.Array_Billboard`)) (`self.HoverOffset`)) true true)
  (switch `/Game/Cards/ECard_State` (`self.cardStateSelection`)
    (:`NewEnumerator1`
      (`SceneComponent.SetWorldScale3D` _card0 (1.0 1.0 1.0)))
    (:`NewEnumerator3`
      (`SceneComponent.SetWorldScale3D` _card0 (1.0 1.0 1.0)))))

(fn `PlaceCardOnBoard`
  (params (PlaceLocation :type "Vector Structure"))
  (returns (ReturnValue :type Boolean))
  (set `self.boardPlaceLocation` PlaceLocation)
  (return false))

(fn `SetCardData`
  (params (RowName :type Name))
  (bind _returnvalue (`|GetDataTableRow` "/Game/Manage/CardsData/DT_SportCards.DT_SportCards" RowName)
    (:`then`
      (set `self.cardSportName` (`KismetTextLibrary.Conv_NameToText` RowName))
      (set `self.cardSportColor` (`.Color_7_F1884BF94702D8EA9AC7B79B54B96B53` (break `/Game/Manage/CardsData/STR_SportCard` _returnvalue)))
      (`self.UpdateCardData`))))

(fn `UpdateCardData`
  (`TextRenderComponent.K2_SetText` (`self.TextRender`) (`KismetTextLibrary.Conv_StringToText` (`|GetEnumeratorNameAsString` (`.Sport_17_38FD1F4B40267EEBD058E8857A4275B9` (break `/Game/Manage/CardsData/STR_SportCard` (`self.STR_SportCard`)))))))

(fn `UserConstructionScript`)