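; Player controller for a sports card matching game, handling click selection and checking for three cards of the same sport.
; On BeginPlay it caches GM_MainMode and enables click events; left clicks trace under the cursor and send FInteractMessage to the hit actor with SelectedCard.
; ControlNCard compares the first three SelectedCardArray sports when SelectedCard equals three, reporting a full match to the game mode.
; F_Drawing is an empty stub.
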(event `self.ReceiveBeginPlay`
  (bind _asgm_main_mode (cast `/Game/Personal/GM_MainMode` (`GameplayStatics.GetGameMode`)))
  (set `self.As GM Main Mode` _asgm_main_mode)
  (set `self.bEnableClickEvents` true))

(event `Key|LeftMouseButton`
  (params (Key :type "Key Structure"))
  (:`Pressed`
    (message `/Game/Personal/BPI_Interaction.F_Interact` (`.HitActor` (`GameplayStatics.BreakHitResult` (`self.GetHitResultUnderCursorByChannel` "TraceTypeQuery1"))) (`self.SelectedCard`))))

(event `ControlNCard`
  (bind _selectedcardarray (`self.SelectedCardArray`))
  (bind _sport (break `/Game/Manage/CardsData/STR_SportCard` (`/Game/Personal/BP_CartaMaster.STR_SportCard` (`|GetArrayItem` _selectedcardarray))))
  (bind _sport_2 (break `/Game/Manage/CardsData/STR_SportCard` (`/Game/Personal/BP_CartaMaster.STR_SportCard` (`|GetArrayItem` _selectedcardarray 1))))
  (if (== (`self.SelectedCard`) 3)
    (if (and (`|EnumEquality` _sport _sport_2) (`|EnumEquality` _sport_2 (`.Sport_17_38FD1F4B40267EEBD058E8857A4275B9` (break `/Game/Manage/CardsData/STR_SportCard` (`/Game/Personal/BP_CartaMaster.STR_SportCard` (`|GetArrayItem` _selectedcardarray 2))))))
      (`/Game/Personal/GM_MainMode.OnSelectedSameCard` (`self.As GM Main Mode`) _sport))))

(fn `F_Drawing`)

(fn `UserConstructionScript`)